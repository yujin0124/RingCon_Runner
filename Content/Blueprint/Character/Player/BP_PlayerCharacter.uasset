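; BP_PlayerCharacter is the player character, steered by Joy-Con motion controls.
; Each Tick, a successful gyroscope read from Joy-Con 1 feeds its X and Y directly into controller yaw and pitch.
; Within that same check, Joy-Con 0 acceleration magnitude above a threshold calls MoveForward and debug-prints the value, so shaking moves the player.
; The construction script hands the character to its ACIKFoot component, apparently for foot IK.
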(event EventBeginPlay)

(event Collision|EventActorBeginOverlap
  (params (OtherActor :type Actor%20Object%20Reference)))

(event EventTick
  (params (DeltaSeconds :type Float%20%28single-precision%29))
  (bind _accelerometer (Class|JoyConPluginBPLibrary|GetJoyConAccelerometer))
  (bind (_success _gyroscope) (Class|JoyConPluginBPLibrary|GetJoyConGyroscope 1))
  (bind _returnvalue (Math|Vector|VectorLength _accelerometer))
  (bind (_x _y) (Math|Vector|BreakVector _gyroscope))
  (if _success
    (Pawn|Input|AddControllerYawInput _x)
    (Pawn|Input|AddControllerPitchInput _y)
    (if (> _returnvalue 1.12)
      (Class|PlayerCharacter|MoveForward 1.0)
      (Development|PrintString (Utilities|String|ToString(Float) _returnvalue)))))

(fn ConstructionScript
  (Variables|/Game/Blueprint/Character/Player/AC_IK_Foot.AC_IK_Foot_C|SetCharacter (Variables|Default|GetAC_IK_Foot) self))