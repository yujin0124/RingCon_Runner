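; Foot IK component that computes left foot, right foot and pelvis offsets to fit the character to the ground.
; Each tick, a complex Camera-channel line trace runs down from capsule-center height at each foot bone's XY to below the capsule.
; Hit distance minus capsule half-height gives each offset, or zero on a miss.
; Offsets are smoothed with FInterpTo, and the pelvis follows the larger foot offset.
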(event EventBeginPlay)

(event EventTick
  (params (DeltaSeconds :type Float%20%28single-precision%29))
  (Variables|Default|SetDelta%20Seconds DeltaSeconds)
  (bind _return_value (CallFunction|TracefromFoot (Variables|Parameters|GetLeftFootName) (Variables|Parameters|GetTrace%20Dist%20Below%20Capsule)))
  (Variables|Default|SetLeftFootOffset (Math|Interpolation|FInterpTo (Variables|Default|GetLeftFootOffset) _return_value (Variables|Default|GetDelta%20Seconds) (Variables|Parameters|GetInterp%20Speed)))
  (bind _return_value_2 (CallFunction|TracefromFoot (Variables|Parameters|GetRightFootName) (Variables|Parameters|GetTrace%20Dist%20Below%20Capsule)))
  (Variables|Default|SetRightFootOffset (Math|Interpolation|FInterpTo (Variables|Default|GetRightFootOffset) _return_value_2 (Variables|Default|GetDelta%20Seconds) (Variables|Parameters|GetInterp%20Speed)))
  (Variables|Default|SetPelvisOffset (Math|Interpolation|FInterpTo (Variables|Default|GetPelvisOffset) (Math|Float|Max(Float) (Variables|Default|GetLeftFootOffset) (Variables|Default|GetRightFootOffset)) (Variables|Default|GetDelta%20Seconds) (Variables|Parameters|GetInterp%20Speed))))

(fn TracefromFoot
  (params (BoneName :type Name) (TraceDistBelowCapsule :type Float%20%28single-precision%29))
  (LocalVariables|SetL_TraceDisBelowCapsule TraceDistBelowCapsule)
  (LocalVariables|SetL_BoneLocation (Transformation|GetSocketLocation (Variables|/Script/Engine.Character|GetMesh (Variables|Default|GetCharacter)) BoneName))
  (LocalVariables|SetL_TraceStartLocation (Math|Vector|MakeVector (.x (LocalVariables|GetL_BoneLocation)) (.y (LocalVariables|GetL_BoneLocation)) (.z (Transformation|GetActorLocation (Variables|Default|GetCharacter)))))
  (LocalVariables|SetL_TraceEndLocation (Math|Vector|MakeVector (.x (LocalVariables|GetL_BoneLocation)) (.y (LocalVariables|GetL_BoneLocation)) (- (.z (Transformation|GetActorLocation (Variables|Default|GetCharacter))) (+ (Components|Capsule|GetScaledCapsuleHalfHeight (Variables|/Script/Engine.Character|GetCapsuleComponent (Variables|Default|GetCharacter))) (LocalVariables|GetL_TraceDisBelowCapsule)))))
  (bind (_outhit _returnvalue) (Collision|LineTraceByChannel (LocalVariables|GetL_TraceStartLocation) (LocalVariables|GetL_TraceEndLocation) "TraceTypeQuery2" true 0 "None"))
  (return (Math|Float|SelectFloat (- (Math|Vector|VectorLength (- (LocalVariables|GetL_TraceStartLocation) (.Location (Collision|BreakHitResult _outhit)))) (Components|Capsule|GetScaledCapsuleHalfHeight (Variables|/Script/Engine.Character|GetCapsuleComponent (Variables|Default|GetCharacter)))) 0.0 _returnvalue)))